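; Inventory component that stores a collection of unique items and broadcasts changes to it.
; TryAddItem rejects items already held, while TryRemoveItem acts only on held items; both return success and fire the OnItemAdded or OnItemRemoved dispatcher.
; CheckForItem and GetLenght expose membership and item count.
; A debug key press on I prints the name of every held item.
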(event Input|KeyboardEvents|DebugKeyI
  (params (Key :type Key%20Structure) (ActionValue :type Input%20Action%20Value%20Structure))
  (:Pressed
    (CallFunction|DebugItems)))

(fn TryAddItem
  (params (ItemToAdd :type Struct%20Item%20Structure%20%28by%20ref%29))
  (if (Utilities|Array|ContainsItem (Variables|Default|GetItems) ItemToAdd)
    (return false)
    (else
      (Utilities|Array|Add (Variables|Default|GetItems) ItemToAdd)
      (Default|CallOnItemAdded ItemToAdd)
      (return true))))

(fn TryRemoveItem
  (params (ItemToRemove :type Struct%20Item%20Structure%20%28by%20ref%29))
  (if (Utilities|Array|ContainsItem (Variables|Default|GetItems) ItemToRemove)
    (bind _returnvalue (Utilities|Array|RemoveItem (Variables|Default|GetItems) ItemToRemove))
    (Default|CallOnItemRemoved ItemToRemove)
    (return _returnvalue)
    (else
      (return false))))

(fn CheckforItem
  (params (ItemToCheck :type Struct%20Item%20Structure%20%28by%20ref%29))
  (return (Utilities|Array|ContainsItem (Variables|Default|GetItems) ItemToCheck)))

(fn DebugItems
  (for _array_element (Variables|Default|GetItems)
    (Development|PrintString (Utilities|String|ToString(Name) (.ItemName (Utilities|Struct|BreakStruct_Item _array_element))))))

(fn GetLenght
  (return (Utilities|Array|Length (Variables|Default|GetItems))))