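; BP_ItemPickup is a world item pickup whose type is chosen by a row selector into DT_Items.
; The construction script sets the mesh from that row and applies a dynamic instance of the AtariColors material to slot 0.
; Interact passes the row to the player's BPC_Inventory through TryAddItem and destroys the actor only on success.
; OnLookMessage returns the row's item name as text.
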(event `/Game/RemDev/PlayerCharacter/Interaction/BPI_Interaction.Interact`
  (bind (_itemselector_datatable _itemselector_rowname) (break `DataTableRowHandle` (`self.ItemSelector`)))
  (bind _returnvalue (`self.GetComponentByClass` (`GameplayStatics.GetPlayerCharacter` 0) "/Game/RemDev/Components/BPC_Inventory.BPC_Inventory_C"))
  (`/Engine/EditorBlueprintResources/StandardMacros.IsValid` _returnvalue
    (:`Is Valid`
      (bind _returnvalue_2 (`|GetDataTableRow` "/Game/RemDev/PlayerCharacter/Inventory/DT_Items.DT_Items" _itemselector_rowname)
        (:`then`
          (bind _success_ (`/Game/RemDev/Components/BPC_Inventory.TryAddItem` _returnvalue _returnvalue_2))
          (if _success_
            (`self.K2_DestroyActor`)))))))

(fn `OnLookMessage`
  (returns (OnLookMessage :type Text))
  (bind (_itemselector_datatable _itemselector_rowname) (break `DataTableRowHandle` (`self.ItemSelector`)))
  (bind _returnvalue (`|GetDataTableRow` "/Game/RemDev/PlayerCharacter/Inventory/DT_Items.DT_Items" _itemselector_rowname)
    (:`then`
      (return (`KismetTextLibrary.Conv_NameToText` (`.ItemName_18_06E734074131D9D044BE4E9AC28BB504` (break `/Game/RemDev/PlayerCharacter/Inventory/Struct_Item` _returnvalue)))))))

(fn `UserConstructionScript`
  (bind (_itemselector_datatable _itemselector_rowname) (break `DataTableRowHandle` (`self.ItemSelector`)))
  (bind _returnvalue (`|GetDataTableRow` "/Game/RemDev/PlayerCharacter/Inventory/DT_Items.DT_Items" _itemselector_rowname)
    (:`then`
      (`StaticMeshComponent.SetStaticMesh` (`self.Mesh`) (`.Mesh_12_7B8399C0460A4001A9B11984D84280A8` (break `/Game/RemDev/PlayerCharacter/Inventory/Struct_Item` _returnvalue)))
      (bind _returnvalue_2 (`PrimitiveComponent.CreateDynamicMaterialInstance` (`self.Mesh`) 0 "/Game/RemDev/ItemMeshes/AtariColors.AtariColors" "None"))
      (`PrimitiveComponent.SetMaterial` (`self.Mesh`) 0 _returnvalue_2))))