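; Player component that holds a supermarket shopping checklist and signals when every item on it is checked.
; GenerateList fills a name-to-checked map with all items data table rows, while GenerateRandomList refills it with random picks from those cached row names.
; CheckItem marks a listed item and runs CheckIfCompleted, which calls OnListCompleted through a DoOnce once all entries are true.
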(fn `CheckIfCompleted`
  (returns (`bIsComplete?` :type Boolean))
  (bind _keys (`BlueprintMapLibrary.Map_Keys` (`self.ItemsChecklistMap`)))
  (for _array_element _keys
    (bind (_value _returnvalue) (`BlueprintMapLibrary.Map_Find` (`self.ItemsChecklistMap`) _array_element))
    (if _value
      (if _returnvalue
        (`KismetSystemLibrary.PrintString` "item checked")
        (else
          (return false)))
      (else
        (return false))))
  (`/Engine/EditorBlueprintResources/StandardMacros.DoOnce` false
    (:`Completed`
      (`self.OnListCompleted`)
      (return true))))

(fn `CheckItem`
  (params (Key :type "Name (by ref)"))
  (bind _itemschecklistmap (`self.ItemsChecklistMap`))
  (if (`BlueprintMapLibrary.Map_Contains` _itemschecklistmap Key)
    (`BlueprintMapLibrary.Map_Add` _itemschecklistmap (`local.Key`) true)
    (`self.CheckIfCompleted`)))

(fn `GenerateList`
  (returns (GeneratedList :type "Array of Name"))
  (bind _outrownames (`DataTableFunctionLibrary.GetDataTableRowNames` (`self.ItemsDataTableRef`)))
  (set `self.DTRowNames` _outrownames)
  (`KismetArrayLibrary.Array_Clear` (`self.GeneratedList`))
  (`BlueprintMapLibrary.Map_Clear` (`self.ItemsChecklistMap`))
  (for _array_element (`self.DTRowNames`)
    (`BlueprintMapLibrary.Map_Add` (`self.ItemsChecklistMap`) _array_element)
    (`KismetArrayLibrary.Array_AddUnique` (`self.GeneratedList`) _array_element))
  (for _array_element_2 (`self.GeneratedList`)
    (`KismetSystemLibrary.PrintString` (`KismetStringLibrary.Conv_NameToString` _array_element_2)))
  (return (`self.GeneratedList`)))

(fn `GenerateRandomList`
  (params (Lenght :type Integer))
  (locals (CurrentlySelectedItemName :type Name))
  (`BlueprintMapLibrary.Map_Clear` (`self.ItemsChecklistMap`))
  (for _ (range (+ Lenght 1))
    (bind _output_get (set `local.CurrentlySelectedItemName` (`|GetArrayItem` (`self.DTRowNames`) (`KismetMathLibrary.RandomInteger` (`KismetArrayLibrary.Array_Length` (`self.DTRowNames`))))))
    (`BlueprintMapLibrary.Map_Add` (`self.ItemsChecklistMap`) _output_get)))

(fn `GetGeneratedList`
  (returns (DTRowNames :type "Array of Name"))
  (return (`self.DTRowNames`)))