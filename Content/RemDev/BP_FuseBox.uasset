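; Fuse box actor with an animated door, a lever and switchable power for a set of lights.
; Door and lever toggle through FlipFlops, using timelines played forward or reversed to lerp pivot rotations, with flags guarding against re-triggering.
; Power toggles independently, setting each light bright or dim and firing OnPowerStateChanged inside the loop, once per light.
; The interaction interface section is unwired.
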(event `ToggleDoor`
  ;[0.3 0.3 0.6] Door Animation
  (if (not (`self.bIsDoorLerping?`))
    (`/Engine/EditorBlueprintResources/StandardMacros.FlipFlop`
      (:`A`
        (`self.OpenDoor`))
      (:`B`
        (`self.CloseDoor`)))))

(event `ToggleLever`
  ;[0.3 0.3 0.6] Lever Animation
  (if (not (`self.bIsLeverLerping?`))
    (`/Engine/EditorBlueprintResources/StandardMacros.FlipFlop`
      (:`A`
        (`self.LeverUp`))
      (:`B`
        (`self.LeverDown`)))))

(event `OpenDoor`
  ;[0.3 0.3 0.6] Door Animation
  (if (not (`self.bIsDoorLerping?`))
    (set `self.bIsDoorLerping?` true)
    (bind (_direction _dooralpha) (`Timeline|DoorTimeline` :!label _label)
      (:`Update`
        (`SceneComponent.K2_SetRelativeRotation` (`self.DoorPivot`) (`KismetMathLibrary.RLerp` (struct) (struct :`Yaw` 160.0) _dooralpha) false false))
      (:`Finished`
        (set `self.bIsDoorLerping?` false)))))

(event `LeverUp`
  ;[0.3 0.3 0.6] Lever Animation
  (if (not (`self.bIsLeverLerping?`))
    (set `self.bIsLeverLerping?` true)
    (bind (_direction _dooralpha) (`Timeline|Timeline` :!label _label_2)
      (:`Update`
        (`SceneComponent.K2_SetRelativeRotation` (`self.LeverPivot`) (`KismetMathLibrary.RLerp` (struct :`Roll` 145.0) (struct) _dooralpha) false false))
      (:`Finished`
        (set `self.bIsLeverLerping?` false)))))

(event `CloseDoor`
  ;[0.3 0.3 0.6] Door Animation
  (if (not (`self.bIsDoorLerping?`))
    (set `self.bIsDoorLerping?` true)
    (goto _label :!via `Reverse`)))

(event `LeverDown`
  ;[0.3 0.3 0.6] Lever Animation
  (if (not (`self.bIsDoorLerping?`))
    (set `self.bIsLeverLerping?` true)
    (goto _label_2 :!via `Reverse`)))

(event `TogglePower`
  (if (`self.bIsPowerOn?`)
    (`self.TurnOffPower`)
    (else
      (`self.TurnOnPower`))))

(event `TurnOnPower`
  (for _array_element _
    (`LightComponent.SetIntensity` (`Light.LightComponent` _array_element) 100.0)
    (bind _output_get (set `self.bIsPowerOn?` true))
    (`self.OnPowerStateChanged` _output_get)))

(event `TurnOffPower`
  (for _array_element _
    (`LightComponent.SetIntensity` (`Light.LightComponent` _array_element) 0.5)
    (bind _output_get (set `self.bIsPowerOn?` false))
    (`self.OnPowerStateChanged` _output_get)))

(fn `UserConstructionScript`)