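; BP_MainDoor is a two-panel sliding door that opens automatically when a Pawn enters its trigger box and closes when the Pawn leaves.
; A timeline lerps the left and right pivots apart sideways, and closing reverses the same timeline.
; An IsLocked flag blocks opening but not closing, and OnLookMessage returns a no-power message while the door is locked.
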(event `OpenDoor`
  (if (not (`self.bIsLocked?`))
    (bind (_direction _alpha) (`Timeline|Timeline` :!label _label)
      (:`Update`
        (`SceneComponent.K2_SetRelativeLocation` (`self.LeftDoorPivot`) (`KismetMathLibrary.VLerp` (0.0 0.0 0.0) (0.0 -200.0 0.0) _alpha) false false)
        (`SceneComponent.K2_SetRelativeLocation` (`self.RightDoorPivot`) (`KismetMathLibrary.VLerp` (0.0 0.0 0.0) (0.0 200.0 0.0) _alpha) false false)))))

(event `CloseDoor`
  (goto _label :!via `Reverse`))

(event `self.Box.OnComponentBeginOverlap`
  (params (OverlappedComponent :type "PrimitiveComponent Object Reference") (OtherActor :type "Actor Object Reference") (OtherComp :type "PrimitiveComponent Object Reference") (OtherBodyIndex :type Integer) (bFromSweep :type Boolean) (SweepResult :type "HitResult Structure (by ref)"))
  (cast `Pawn` OtherActor)
  (`self.OpenDoor`))

(event `self.Box.OnComponentEndOverlap`
  (params (OverlappedComponent :type "PrimitiveComponent Object Reference") (OtherActor :type "Actor Object Reference") (OtherComp :type "PrimitiveComponent Object Reference") (OtherBodyIndex :type Integer))
  (cast `Pawn` OtherActor)
  (`self.CloseDoor`))

(fn `OnLookMessage`
  (returns (OnLookMessage :type Text))
  (if (`self.bIsLocked?`)
    (return "The door wont open without power")))

(fn `UserConstructionScript`)