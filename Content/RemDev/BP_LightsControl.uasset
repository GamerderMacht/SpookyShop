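; BP_LightsControl is an interactable light switch that toggles a set of lights between bright and dim.
; Interact calls ToggleLights, which checks AreLightsOn and runs TurnOnLights or TurnOffLights.
; Both events loop over the Lights array to set each light component's intensity and update the flag, with off leaving a faint glow.
; OnLookMessage supplies the "Light control" label.
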(event `ToggleLights`
  (if (`self.bAreLightsOn?`)
    (`self.TurnOffLights`)
    (else
      (`self.TurnOnLights`))))

(event `TurnOnLights`
  (for _array_element (`self.Lights`)
    (`LightComponent.SetIntensity` (`Light.LightComponent` _array_element) 100.0)
    (set `self.bAreLightsOn?` true)))

(event `TurnOffLights`
  (for _array_element (`self.Lights`)
    (`LightComponent.SetIntensity` (`Light.LightComponent` _array_element) 0.5)
    (set `self.bAreLightsOn?` false)))

(event `/Game/RemDev/PlayerCharacter/Interaction/BPI_Interaction.Interact`
  (`self.ToggleLights`))

(fn `OnLookMessage`
  (returns (OnLookMessage :type Text))
  (return "Light control"))

(fn `UserConstructionScript`)