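; BP_CarInteractable is the player's car, an interactable that shows "My car" on look and can end the game.
; On BeginPlay it caches BP_GameStateManager, then switches on the current game state when interacted with.
; The initial state shows dialogue, while Paid Items, Asked for Milk and Lights Out each open WB_GameOver with a different ending.
; Ending screens switch input to UI-only and show the mouse cursor.
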(event `self.ReceiveBeginPlay`
  (bind _returnvalue (`GameplayStatics.GetActorOfClass` "/Game/RemDev/Actors/BP_GameStateManager.BP_GameStateManager_C"))
  (set `self.StateManagerRef` _returnvalue))

(event `/Game/RemDev/PlayerCharacter/Interaction/BPI_Interaction.Interact`
  (bind _returnvalue (`GameplayStatics.GetPlayerController` 0))
  (bind _returnvalue_2 (`GameplayStatics.GetPlayerController` 0))
  (bind _returnvalue_3 (`GameplayStatics.GetPlayerController` 0))
  (bind _currentgamestate (`/Game/RemDev/Actors/BP_GameStateManager.GetCurrentGameState` (`self.StateManagerRef`)))
  (switch `/Game/RemDev/Actors/SpookyGameStates` _currentgamestate
    (:`NewEnumerator0`
      (`/Game/RemDev/UI/BPFL_UIHelper.ShowDialogue` 5))
    (:`NewEnumerator1`
      ;[1 1 1] Show Game Over 2
      (bind _returnvalue_4 (`|CreateWidget` "/Game/RemDev/WB_GameOver.WB_GameOver_C" _returnvalue))
      (`UserWidget.AddToViewport` _returnvalue_4 0)
      (`/Game/RemDev/WB_GameOver.SetEndingInfo` _returnvalue_4 2 "Survived")
      (`WidgetBlueprintLibrary.SetInputMode_UIOnlyEx` _returnvalue _returnvalue_4 "DoNotLock" true)
      (set `PlayerController.bShowMouseCursor` true _returnvalue))
    (:`NewEnumerator2`
      ;[1 1 1] Show Game Over 3
      (bind _returnvalue_5 (`|CreateWidget` "/Game/RemDev/WB_GameOver.WB_GameOver_C" _returnvalue_3))
      (`UserWidget.AddToViewport` _returnvalue_5 0)
      (`/Game/RemDev/WB_GameOver.SetEndingInfo` _returnvalue_5 3 "Shoplifter")
      (`WidgetBlueprintLibrary.SetInputMode_UIOnlyEx` _returnvalue_3 _returnvalue_5 "DoNotLock" true)
      (set `PlayerController.bShowMouseCursor` true _returnvalue_3))
    (:`NewEnumerator3`
      ;[1 1 1] Show Game Over 4
      (bind _returnvalue_6 (`|CreateWidget` "/Game/RemDev/WB_GameOver.WB_GameOver_C" _returnvalue_2))
      (`UserWidget.AddToViewport` _returnvalue_6 0)
      (`/Game/RemDev/WB_GameOver.SetEndingInfo` _returnvalue_6 4 "Lucky")
      (`WidgetBlueprintLibrary.SetInputMode_UIOnlyEx` _returnvalue_2 _returnvalue_6 "DoNotLock" true)
      (set `PlayerController.bShowMouseCursor` true _returnvalue_2))))

(fn `OnLookMessage`
  (returns (OnLookMessage :type Text))
  (return "My car"))

(fn `UserConstructionScript`)